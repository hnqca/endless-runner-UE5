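; BP_Floor is a runner-game floor tile that fills itself with random obstacles, coins and occasional power-ups.
; Its construction script builds arrow-marked points along each lane, shuffles them and attaches child actors.
; Power-up rolls wait until the GameMode's FloorCount passes a threshold, then reset it even if nothing spawns.
; Runner overlap asks the GameMode to extend the floor and slightly raises clamped walk speed; GetAttachPoint exposes the arrow transform.
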(event OnComponentBeginOverlap(Collision)
  (params (OverlappedComponent :type Primitive%20Component%20Object%20Reference) (OtherActor :type Actor%20Object%20Reference) (OtherComp :type Primitive%20Component%20Object%20Reference) (OtherBodyIndex :type Integer) (bFromSweep :type Boolean) (SweepResult :type Hit%20Result%20Structure%20%28by%20ref%29))
  (bind _asbp_runner_character (Utilities|Casting|CastToBP_RunnerCharacter OtherActor))
  (bind _asbp_runner_game_mode (Utilities|Casting|CastToBP_RunnerGameMode (Game|GetGameMode)))
  (Default|ExtendFloor _asbp_runner_game_mode)
  ;[1 1 1] Change Speed
  (bind _output_get (Variables|/Script/Engine.CharacterMovementComponent|SetMaxWalkSpeed (Variables|/Script/Engine.Character|GetCharacterMovement _asbp_runner_character) (Math|Float|Clamp(Float) (* (Variables|/Script/Engine.CharacterMovementComponent|GetMaxWalkSpeed (Variables|/Script/Engine.Character|GetCharacterMovement _asbp_runner_character)) 1.005) 7e+02 1.5e+03))))

(event Collision|EventActorBeginOverlap
  (params (OtherActor :type Actor%20Object%20Reference)))

(event EventTick
  (params (DeltaSeconds :type Float%20%28single-precision%29)))

(fn ConstructionScript
  (CallFunction|SetupSpawnPoints)
  (CallFunction|SpawnObstacles)
  (CallFunction|CoinSpawnPoints)
  (CallFunction|SpawnCoins)
  (CallFunction|PowerUpsSpawnPoints)
  (CallFunction|SpawnPowerUps))

(fn GetAttachPoint
  (return (Transformation|GetWorldTransform (Variables|Default|GetArrow))))

(fn SetupSpawnPoints
  (for _array_element (Variables|Default|GetlanePosition)
    (for _index (range 0 1)
      (bind _returnvalue (AddComponent|AddArrowComponent false (Math|Transform|MakeTransform (Math|Vector|MakeVector (* _index 6.5e+02) _array_element 0.0))))
      (Utilities|Array|Add (Variables|Default|GetspawnPoints) (Transformation|GetWorldTransform _returnvalue)))))

(fn SpawnObstacles
  (bind _output_get (Variables|Default|SetrandomSpawnPoints (Variables|Default|GetspawnPoints)))
  (Utilities|Array|Shuffle _output_get)
  (for _index (range 0 (Math|Random|RandomIntegerinRange 0 2))
    (switch int (Math|Random|RandomIntegerinRange 0 4)
      (:0
        (AddComponent|AddChildActorComponent false (Math|Transform|MakeRelativeTransform (Utilities|Array|Get(acopy) (Variables|Default|GetrandomSpawnPoints) _index) (Transformation|GetActorTransform))))
      (:1
        (AddComponent|AddChildActorComponent false (Math|Transform|MakeRelativeTransform (Utilities|Array|Get(acopy) (Variables|Default|GetrandomSpawnPoints) _index) (Transformation|GetActorTransform))))
      (:2
        (AddComponent|AddChildActorComponent false (Math|Transform|MakeRelativeTransform (Utilities|Array|Get(acopy) (Variables|Default|GetrandomSpawnPoints) _index) (Transformation|GetActorTransform))))
      (:3
        (AddComponent|AddChildActorComponent false (Math|Transform|MakeRelativeTransform (Utilities|Array|Get(acopy) (Variables|Default|GetrandomSpawnPoints) _index) (Transformation|GetActorTransform))))
      (:4
        (AddComponent|AddChildActorComponent false (Math|Transform|MakeRelativeTransform (Utilities|Array|Get(acopy) (Variables|Default|GetrandomSpawnPoints) _index) (Transformation|GetActorTransform)))))))

(fn CoinSpawnPoints
  (for _array_element (Variables|Default|GetlanePosition)
    (for _index (range 0 9)
      (bind _returnvalue (AddComponent|AddArrowComponent false (Math|Transform|MakeTransform (Math|Vector|MakeVector (* _index 75.0) _array_element 0.0))))
      (Components|Arrow|SetArrowColor(LinearColor) _returnvalue "(R=1.000000,G=0.685823,B=0.000000,A=1.000000)")
      (Utilities|Array|Add (Variables|Default|GetcoinSpawnPoints) (Transformation|GetWorldTransform _returnvalue)))))

(fn SpawnCoins
  (bind _output_get (Variables|Default|SetrandomSpawnPoints (Variables|Default|GetcoinSpawnPoints)))
  (Utilities|Array|Shuffle _output_get)
  (for _index (range 0 (Math|Random|RandomIntegerinRange 1 8))
    (AddComponent|AddChildActorComponent false (Math|Transform|MakeRelativeTransform (Utilities|Array|Get(acopy) (Variables|Default|GetrandomSpawnPoints) _index) (Transformation|GetActorTransform)))))

(fn PowerUpsSpawnPoints
  (for _array_element (Variables|Default|GetlanePosition)
    (for _index (range 1 2)
      (bind _returnvalue (AddComponent|AddArrowComponent false (Math|Transform|MakeTransform (Math|Vector|MakeVector (* _index 2.5e+02) _array_element 0.0))))
      (Components|Arrow|SetArrowColor(LinearColor) _returnvalue "(R=1.000000,G=0.000000,B=0.019224,A=1.000000)")
      (Utilities|Array|Add (Variables|Default|GetpowerUpsSpawnPoints) (Transformation|GetWorldTransform _returnvalue)))))

(fn SpawnPowerUps
  (bind _asbp_runner_game_mode (Utilities|Casting|CastToBP_RunnerGameMode (Game|GetGameMode)))
  (if (> (Variables|/Game/Game/Blueprints/BP_RunnerGameMode.BP_RunnerGameMode_C|GetfloorCount _asbp_runner_game_mode) 5)
    (bind _output_get (Variables|Default|SetrandomSpawnPoints (Variables|Default|GetpowerUpsSpawnPoints)))
    (Utilities|Array|Shuffle _output_get)
    (switch int (Math|Random|RandomIntegerinRange 0 10)
      (:0
        (AddComponent|AddChildActorComponent false (Math|Transform|MakeRelativeTransform (Utilities|Array|Get(acopy) (Variables|Default|GetrandomSpawnPoints)) (Transformation|GetActorTransform))))
      (:1
        (AddComponent|AddChildActorComponent false (Math|Transform|MakeRelativeTransform (Utilities|Array|Get(acopy) (Variables|Default|GetrandomSpawnPoints)) (Transformation|GetActorTransform))))
      (:2
        _)
      (:3
        _)
      (:4
        _)
      (:5
        _)
      (:6
        _)
      (:7
        _)
      (:8
        _)
      (:9
        _)
      (:10
        _))
    (Variables|/Game/Game/Blueprints/BP_RunnerGameMode.BP_RunnerGameMode_C|SetfloorCount _asbp_runner_game_mode 0)))