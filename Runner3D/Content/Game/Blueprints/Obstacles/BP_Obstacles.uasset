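; BP_Obstacles is an obstacle actor that kills the runner character on contact.
; When its DeathCollision component begins overlapping a BP_RunnerCharacter, it confirms that the character's capsule overlaps the obstacle.
; It then calls Death and pauses the game after a short delay, unless the character is sliding and the obstacle is flagged as ObstacleSlider.
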(event OnComponentBeginOverlap(deathCollision)
  (params (OverlappedComponent :type Primitive%20Component%20Object%20Reference) (OtherActor :type Actor%20Object%20Reference) (OtherComp :type Primitive%20Component%20Object%20Reference) (OtherBodyIndex :type Integer) (bFromSweep :type Boolean) (SweepResult :type Hit%20Result%20Structure%20%28by%20ref%29))
  (bind _asbp_runner_character (Utilities|Casting|CastToBP_RunnerCharacter OtherActor))
  (if (Collision|IsOverlappingActor (Variables|/Script/Engine.Character|GetCapsuleComponent _asbp_runner_character) self :!class /Script/Engine.PrimitiveComponent)
    (if (not (and (Variables|/Game/Game/Blueprints/Characters/BP_RunnerCharacter.BP_RunnerCharacter_C|GetisSliding? _asbp_runner_character) (Variables|Default|GetobstacleSlider?)))
      (Default|Death _asbp_runner_character)
      (Utilities|FlowControl|Delay 3.0)
      (Game|SetGamePaused true))))

(fn ConstructionScript)