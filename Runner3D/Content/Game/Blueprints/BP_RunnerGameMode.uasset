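; Game mode for a runner game that builds a rolling floor of BP_Floor tiles and sets the match objective.
; BeginPlay spawns the initial tiles and picks a random row name from DT_Objectives as the current objective.
; AddFloor chains each tile to the previous one's attach point and increments the floor count.
; ExtendFloor adds a tile and destroys the oldest once the array exceeds the initial count plus a small buffer.
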(event EventBeginPlay
  (Utilities|FlowControl|Sequence
    (:then_0
      (for _index (range 0 (- (Variables|Default|GetnumberOfTiles) 1))
        (CallFunction|AddFloor)))
    (:then_1
      ;[1 1 1 1 20] Selects a random objective for the player at the beginning of the match.
      (bind _outrownames (DataTable|GetDataTableRowNames "/Game/Game/Blueprints/DataTables/DT_Objectives.DT_Objectives"))
      (Variables|Default|SetcurrentObjective (.OutItem (Utilities|Array|Random _outrownames))))))

(fn ConstructionScript)

(fn AddFloor
  (bind _returnvalue (Game|SpawnActorfromClass "/Game/Game/Blueprints/Floor/BP_Floor.BP_Floor_C" (Variables|Default|GetfloorAttachPoint) "Undefined" "MultiplyWithRoot" 0 0))
  (bind _returnvalue_2 (Default|GetAttachPoint _returnvalue))
  (Variables|Default|SetfloorAttachPoint _returnvalue_2)
  (Utilities|Array|Add (Variables|Default|GetfloorTiles) _returnvalue)
  (bind _result (Math|Integer|IncrementInt (Variables|Default|GetfloorCount))
    (:%20%20
      (Variables|Default|SetfloorCount _result))))

(fn ExtendFloor
  (bind _floortiles (Variables|Default|GetfloorTiles))
  (bind _output (Utilities|Array|Get(acopy) _floortiles))
  (CallFunction|AddFloor)
  (if (> (Utilities|Array|Length (Variables|Default|GetfloorTiles)) (+ (Variables|Default|GetnumberOfTiles) 2))
    (Actor|DestroyActor _output)
    (Utilities|Array|RemoveItem _floortiles _output)))