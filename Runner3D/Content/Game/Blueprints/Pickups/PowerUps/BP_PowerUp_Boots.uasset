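; BP_PowerUp_Boots is a runner pickup that turns on the boots power-up when the player touches it.
; Overlap of its collision casts to BP_RunnerCharacter, then once increments the collected boots count, hides itself, enables the power-up and destroys itself.
; A character reference cached on BeginPlay lets TotalCurrentCompletedMissionByPlayer report that boots count as mission progress.
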(event OnComponentBeginOverlap(collisionColectBonus)
  (params (OverlappedComponent :type Primitive%20Component%20Object%20Reference) (OtherActor :type Actor%20Object%20Reference) (OtherComp :type Primitive%20Component%20Object%20Reference) (OtherBodyIndex :type Integer) (bFromSweep :type Boolean) (SweepResult :type Hit%20Result%20Structure%20%28by%20ref%29))
  (bind _asbp_runner_character (Utilities|Casting|CastToBP_RunnerCharacter OtherActor))
  (Utilities|FlowControl|DoOnce false
    (:Completed
      (bind _result (Math|Integer|IncrementInt (Variables|/Game/Game/Blueprints/Characters/BP_RunnerCharacter.BP_RunnerCharacter_C|GetamountCollectedBoots _asbp_runner_character))
        (:%20%20
          (Variables|/Game/Game/Blueprints/Characters/BP_RunnerCharacter.BP_RunnerCharacter_C|SetamountCollectedBoots _asbp_runner_character _result)
          (Rendering|SetActorHiddenInGame true)
          (Default|On/offBootsPowerUp _asbp_runner_character true)
          (Actor|DestroyActor))))))

(event EventBeginPlay
  (bind _returnvalue (Actor|GetActorOfClass "/Game/Game/Blueprints/Characters/BP_RunnerCharacter.BP_RunnerCharacter_C"))
  (Variables|Default|SetAs%20BP%20Runner%20Character _returnvalue))

(fn ConstructionScript)

(fn TotalCurrentCompletedMissionbyPlayer
  (return (Variables|/Game/Game/Blueprints/Characters/BP_RunnerCharacter.BP_RunnerCharacter_C|GetamountCollectedBoots (Variables|Default|GetAs%20BP%20Runner%20Character))))